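; Coffin Blueprint that opens and releases a zombie when an actor overlaps it.
; BeginPlay hides the CoffinPCube4 mesh; on overlap it destroys CoffinTop and Box, reveals that mesh and plays an attached opening sound.
; It spawns AI_Zombie with BT_Zombie at Box1's center of mass, then destroys Box1.
; The overlap has no actor filter, and a leftover SpawnActor node never runs.
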(event `self.ReceiveBeginPlay`
  (`SceneComponent.SetHiddenInGame` (`self.Coffin_pCube4`) true false))

(event `self.ReceiveActorBeginOverlap`
  (params (OtherActor :type "Actor Object Reference"))
  (bind _coffin_pcube4 (`self.Coffin_pCube4`))
  (`ActorComponent.K2_DestroyComponent` (`self.Coffin_Top`))
  (`ActorComponent.K2_DestroyComponent` (`self.Box`))
  (`SceneComponent.SetHiddenInGame` _coffin_pcube4 false false)
  (`GameplayStatics.SpawnSoundAttached` "/Game/Coffin_Open_Noise.Coffin_Open_Noise" _coffin_pcube4 "None" (0.0 0.0 0.0) (struct) "KeepRelativeOffset" false 1.0 1.0 0.0 null null)
  (`AIBlueprintHelperLibrary.SpawnAIFromClass` "/Game/FPS_Game/Blueprints/Bonus/AI/AI_Zombie.AI_Zombie_C" "/Game/FPS_Game/Blueprints/Bonus/AI/Zombie/BT_Zombie.BT_Zombie" (`PrimitiveComponent.GetCenterOfMass` (`self.Box1`) "None") (struct) true null)
  (`ActorComponent.K2_DestroyComponent` (`self.Box1`)))

(fn `UserConstructionScript`)