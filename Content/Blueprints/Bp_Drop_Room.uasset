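; Drop room actor with a DropPlatform that moves while something overlaps it.
; Beginning an overlap plays the Move timeline, which sets the platform's relative location without sweep, and ending the overlap reverses the timeline.
; Neither overlap event filters by the other actor.
; An unconnected Delay and a second timeline branch with a Box overlap check never run.
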(event `self.ReceiveActorBeginOverlap`
  (params (OtherActor :type "Actor Object Reference"))
  (bind (_direction _newtrack_0) (`Timeline|Move` :`NewTime` 0.0 :!label _label)
    (:`Update`
      (`SceneComponent.K2_SetRelativeLocation` (`self.Drop Platform`) _newtrack_0 false false))))

(event `self.ReceiveActorEndOverlap`
  (params (OtherActor :type "Actor Object Reference"))
  (goto _label :!via `Reverse`))

(fn `UserConstructionScript`)